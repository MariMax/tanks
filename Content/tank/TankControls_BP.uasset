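; Tank controller Blueprint that sets up the player's aiming crosshair HUD when play begins.
; BeginPlay creates an AimPoint widget, adds it to the viewport and copies the crosshair's canvas anchor minimum into CrossHairXPosition and CrossHairYPosition.
; It then hands the controlled tank's TankAimingComponent to the widget as a reference, linking the HUD to that tank's aiming.
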(event `self.ReceiveBeginPlay`
  (bind _returnvalue (`|CreateWidget` "/Game/UI/AimPoint.AimPoint_C"))
  (`|ExecutionSequence`
    (:`then_0`
      (`UserWidget.AddToViewport` _returnvalue 0)
      (bind _ascanvas_panel_slot (cast `CanvasPanelSlot` (`Widget.Slot` (`/Game/UI/AimPoint.CrossHair` _returnvalue))))
      (bind (_x _y) (`KismetMathLibrary.BreakVector2D` (`.Minimum` (break `Anchors` (`CanvasPanelSlot.GetAnchors` _ascanvas_panel_slot)))))
      (set `self.crossHairXPosition` _x)
      (set `self.crossHairYPosition` _y))
    (:`then_1`
      (set `/Game/UI/AimPoint.Aiming Component BP Ref` (`Tank.TankAimingComponent` (`self.GetControlledTank`)) _returnvalue))))

(fn `UserConstructionScript`)