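; Player-controlled tank pawn Blueprint that handles aiming, firing and track-based movement.
; BeginPlay wires the track meshes into TankMovement and the barrel and turret into TankAiming, which also handles firing.
; Aim axes rotate an azimuth gimbal and spring arm.
; Throttle keys play or reverse timelines to ramp speed values, which Tick sums into forward and rotation intents for TankMovement.
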(event `self.ReceiveBeginPlay`
  (`TankMovementComponent.InitTracks` (`self.TankMovement`) (`self.Left Track`) (`self.Right Track`))
  (`TankAimingComponent.InitAimingComponent` (`self.TankAiming`) (`self.TankBarrel`) (`self.TankTurret`)))

(event `InputAxis|AimAzimuth`
  (params (AxisValue :type "Float (single-precision)"))
  ;[1 1 1] Aim input binding
  (`SceneComponent.K2_AddLocalRotation` (`self.Azimuth Gimble`) (`KismetMathLibrary.MakeRotator` 0.0 0.0 AxisValue) false false))

(event `InputAxis|AimAltitude`
  (params (AxisValue :type "Float (single-precision)"))
  ;[1 1 1] Aim input binding
  (`SceneComponent.K2_AddLocalRotation` (`self.SpringArm`) (`KismetMathLibrary.MakeRotator` 0.0 AxisValue) false false))

(event `InputAction|Fire`
  (params (Key :type "Key Structure"))
  ;[1 1 1] Aim input binding
  (:`Pressed`
    (`TankAimingComponent.Fire` (`self.TankAiming`))))

(event `InputAction|ForwardThrottle`
  (params (Key :type "Key Structure"))
  ;[1 1 1] Navigation bindings
  (:`Pressed`
    (bind (_direction _speed) (`Timeline|Forward Speed Change` :!label _label)
      (:`Update`
        (set `self.ForwardSpeed` _speed))))
  (:`Released`
    (goto _label :!via `Reverse`)))

(event `InputAction|RightThrottle`
  (params (Key :type "Key Structure"))
  ;[1 1 1] Navigation bindings
  (:`Pressed`
    (bind (_direction _speed) (`Timeline|Right Speed Change` :!label _label_2)
      (:`Update`
        (set `self.RightSpeed` _speed))))
  (:`Released`
    (goto _label_2 :!via `Reverse`)))

(event `InputAction|LeftThrottle`
  (params (Key :type "Key Structure"))
  ;[1 1 1] Navigation bindings
  (:`Pressed`
    (bind (_direction _speed) (`Timeline|Timeline_0` :!label _label_3)
      (:`Update`
        (set `self.Left Speed` _speed))))
  (:`Released`
    (goto _label_3 :!via `Reverse`)))

(event `InputAction|BackThrottle`
  (params (Key :type "Key Structure"))
  ;[1 1 1] Navigation bindings
  (:`Pressed`
    (bind (_direction _speed) (`Timeline|Back Speed Change` :!label _label_4)
      (:`Update`
        (set `self.BackSpeed` _speed))))
  (:`Released`
    (goto _label_4 :!via `Reverse`)))

(event `self.ReceiveTick`
  (params (DeltaSeconds :type "Float (single-precision)"))
  ;[1 1 1] Navigation bindings
  (`TankMovementComponent.IntendMoveForward` (`self.TankMovement`) (+ (`self.ForwardSpeed`) (`self.BackSpeed`)))
  (`TankMovementComponent.IntendRotate` (`self.TankMovement`) (+ (`self.Left Speed`) (`self.RightSpeed`))))

(fn `UserConstructionScript`)